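; BP_Soldier_01 is a player-controlled soldier pawn that moves along fixed world axes and takes its facing direction from mouse motion.
; Forward/back and left/right axis inputs drive movement on world X and Y, independent of facing.
; Each tick, GetMouseVelocity divides mouse delta by delta time, and UpdatePlayerRotation converts it with atan2 into the controller's yaw.
; IsMouseDeadZone is an empty stub, so no dead zone filters this input.
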(event `self.ReceiveTick`
  (params (DeltaSeconds :type "Float (single-precision)"))
  (`self.Update Player Rotation`))

(event `InputAxis|MoveForwardBack`
  (params (AxisValue :type "Float (single-precision)"))
  (`self.AddMovementInput` (1.0 0.0 0.0) AxisValue))

(event `InputAxis|MoveLeftRight`
  (params (AxisValue :type "Float (single-precision)"))
  (`self.AddMovementInput` (0.0 1.0 0.0) AxisValue))

(fn `GetMouseVelocity`
  (returns (ReturnValue :type "Vector2D Structure"))
  (bind (_deltax _deltay) (`PlayerController.GetInputMouseDelta` (`GameplayStatics.GetPlayerController` 0)))
  (return (/ (`KismetMathLibrary.MakeVector2D` _deltax _deltay) (`GameplayStatics.GetWorldDeltaSeconds`))))

(fn `IsMouseDeadZone`)

(fn `Update Player Rotation`
  (bind (_returnvalue_x _returnvalue_y) (`KismetMathLibrary.BreakVector2D` (`self.GetMouseVelocity`)))
  (`Controller.SetControlRotation` (`GameplayStatics.GetPlayerController` 0) (`KismetMathLibrary.MakeRotator` 0.0 0.0 (`KismetMathLibrary.DegAtan2` _returnvalue_x _returnvalue_y))))

(fn `UserConstructionScript`)